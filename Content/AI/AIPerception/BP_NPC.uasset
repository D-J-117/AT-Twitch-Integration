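; Enemy NPC actor in the AIPerception folder that reports its defeat to the game instance.
; BeginPlay caches the third-person game instance, and DamageNPC increments its enemies-defeated count, then destroys the actor.
; A disconnected, never-executed chain would alternate the Blackboard "Active" flag after a delay and stop controller movement when inactive.
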(event `self.ReceiveBeginPlay`
  ;[0 0 0] Gets Game Instance for later use
  (bind _asgi_third_person_game_instance (cast `/Game/ThirdPerson/Blueprints/GI_ThirdPersonGameInstance` (`GameplayStatics.GetGameInstance`)))
  (set `self.As GI Third Person Game Instance` _asgi_third_person_game_instance))

(event `self.ReceiveTick`
  (params (DeltaSeconds :type "Float (single-precision)")))

(event `Damage NPC`
  (bind _as_gi_third_person_game_instance (`self.As GI Third Person Game Instance`))
  (`/Game/ThirdPerson/Blueprints/GI_ThirdPersonGameInstance.UpdateEnemiesDefeated` _as_gi_third_person_game_instance (+ (`/Game/ThirdPerson/Blueprints/GI_ThirdPersonGameInstance.GetEnemiesDefeated` _as_gi_third_person_game_instance) 1))
  (`self.K2_DestroyActor`))

(fn `UserConstructionScript`)