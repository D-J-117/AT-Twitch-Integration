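; BP_NPC_Spawner is a voting-driven spawner that creates enemy NPCs at its own transform.
; It caches the third-person game instance on BeginPlay, then on Tick checks whether enemies can spawn and, after a one-second delay, reads the vote winner.
; The winner selects BP_NPC or BP_NPC_Var_1, with a tie picking one at random, and spawning ignores collisions.
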(event `self.ReceiveBeginPlay`
  ;[0 0 0] Gets Game Instance for later use
  (bind _asgi_third_person_game_instance (cast `/Game/ThirdPerson/Blueprints/GI_ThirdPersonGameInstance` (`GameplayStatics.GetGameInstance`)))
  (set `self.As GI Third Person Game Instance` _asgi_third_person_game_instance))

(event `self.ReceiveTick`
  (params (DeltaSeconds :type "Float (single-precision)"))
  (if (`/Game/ThirdPerson/Blueprints/GI_ThirdPersonGameInstance.Can Spawn Enemies` (`self.As GI Third Person Game Instance`))
    (`KismetSystemLibrary.Delay` 1.0)
    (switch `int` (`/Game/ThirdPerson/Blueprints/GI_ThirdPersonGameInstance.Get Vote Winner` (`self.As GI Third Person Game Instance`))
      (:`0`
        ;[0 0 0] Tie results in random outcome
        (if (`KismetMathLibrary.RandomBool`)
          (`|SpawnActorFromClass` "/Game/AI/AIPerception/BP_NPC.BP_NPC_C" (`self.GetTransform`) "AlwaysSpawn" "MultiplyWithRoot" null null :!label _label)
          (else
            (`|SpawnActorFromClass` "/Game/AI/AIPerception/BP_NPC_Var_1.BP_NPC_Var_1_C" (`self.GetTransform`) "AlwaysSpawn" "MultiplyWithRoot" null null :!label _label_2))))
      (:`1`
        (goto _label))
      (:`2`
        (goto _label_2)))))

(fn `UserConstructionScript`)