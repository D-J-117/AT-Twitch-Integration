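; Spawner actor that spawns one of two temporary enemy types at its own transform based on the result of a player vote.
; It caches the third-person game instance on BeginPlay and polls it every Tick for vote type 3 (commented as Item) with a valid winner.
; The winner picks the enemy class, with a tie choosing randomly.
; A Spawned flag limits it to one spawn until that vote condition clears.
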(event `self.ReceiveBeginPlay`
  ;[0 0 0] Gets Game Instance for later use
  (bind _asgi_third_person_game_instance (cast `/Game/ThirdPerson/Blueprints/GI_ThirdPersonGameInstance` (`GameplayStatics.GetGameInstance`)))
  (set `self.As GI Third Person Game Instance` _asgi_third_person_game_instance))

(event `self.ReceiveTick`
  (params (DeltaSeconds :type "Float (single-precision)"))
  (bind _as_gi_third_person_game_instance (`self.As GI Third Person Game Instance`))
  (if (and (== (`/Game/ThirdPerson/Blueprints/GI_ThirdPersonGameInstance.Get Current Vote Type` _as_gi_third_person_game_instance) 3) (!= (`/Game/ThirdPerson/Blueprints/GI_ThirdPersonGameInstance.Get Vote Winner` _as_gi_third_person_game_instance) -1))
    (if (not (`self.Spawned`))
      (switch `int` (`/Game/ThirdPerson/Blueprints/GI_ThirdPersonGameInstance.Get Vote Winner` (`self.As GI Third Person Game Instance`))
        (:`0`
          ;[0 0 0] Tie results in random outcome
          (if (`KismetMathLibrary.RandomBool`)
            (`|SpawnActorFromClass` "/Game/VotingObjects/BP_Enemy_Temp_1.BP_Enemy_Temp_1_C" (`self.GetTransform`) "AlwaysSpawn" "MultiplyWithRoot" null null :!label _label)
            (set `self.Spawned` true)
            (else
              (`|SpawnActorFromClass` "/Game/VotingObjects/BP_Enemy_Temp_2.BP_Enemy_Temp_2_C" (`self.GetTransform`) "AlwaysSpawn" "MultiplyWithRoot" null null :!label _label_2)
              (set `self.Spawned` true))))
        (:`1`
          (goto _label))
        (:`2`
          (goto _label_2))))
    (else
      (set `self.Spawned` false))))

(fn `UserConstructionScript`)