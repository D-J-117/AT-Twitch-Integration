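; Level portal actor that sends the player to the next level chosen by a vote.
; Each tick it polls the game instance, activating and showing its effect only when progression is allowed and the required vote type has a winner.
; Player overlap opens the winning level, mapped from the Levels enum name, or a random one on a tie, then tells the game instance to progress.
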(event `self.ReceiveBeginPlay`
  ;[0 0 0] Gets Game Instance for later use
  (bind _asgi_third_person_game_instance (cast `/Game/ThirdPerson/Blueprints/GI_ThirdPersonGameInstance` (`GameplayStatics.GetGameInstance`)))
  (set `self.As GI Third Person Game Instance` _asgi_third_person_game_instance))

(event `self.ReceiveTick`
  (params (DeltaSeconds :type "Float (single-precision)"))
  (bind _as_gi_third_person_game_instance (`self.As GI Third Person Game Instance`))
  (if (`/Game/ThirdPerson/Blueprints/GI_ThirdPersonGameInstance.Get Can Progress Level` (`self.As GI Third Person Game Instance`))
    (if (and (== (`/Game/ThirdPerson/Blueprints/GI_ThirdPersonGameInstance.Get Current Vote Type` _as_gi_third_person_game_instance) 1) (!= (`/Game/ThirdPerson/Blueprints/GI_ThirdPersonGameInstance.Get Vote Winner` _as_gi_third_person_game_instance) -1))
      (set `self.Active` true)
      (`SceneComponent.SetVisibility` (`self.Effect`) true false)
      (else
        (set `self.Active` false :!label _label)
        (`SceneComponent.SetVisibility` (`self.Effect`) false false)))
    (else
      (goto _label))))

(event `self.ReceiveActorBeginOverlap`
  (params (OtherActor :type "Actor Object Reference"))
  ;[0 0 0] Checks if there is a valid vote winner.
  (if (`self.Active`)
    (cast `/Game/ThirdPerson/Blueprints/BP_ThirdPersonCharacter` OtherActor)
    (if (!= (`/Game/ThirdPerson/Blueprints/GI_ThirdPersonGameInstance.Get Vote Winner` (`self.As GI Third Person Game Instance`)) -1)
      ;[0 0 0] If vote is a tie, outcome is random
      (if (== (`/Game/ThirdPerson/Blueprints/GI_ThirdPersonGameInstance.Get Vote Winner` (`self.As GI Third Person Game Instance`)) 0)
        (`GameplayStatics.OpenLevel` (`KismetStringLibrary.Conv_StringToName` (`|GetEnumeratorNameAsString` (cast `/Game/VotingObjects/Enums/Enum_Levels` (`KismetMathLibrary.Conv_IntToByte` (`KismetMathLibrary.RandomIntegerInRange` 0 (- (enumcount `/Game/VotingObjects/Enums/Enum_Levels`) 1)))))))
        (else
          ;[0 0 0] Otherwise the vote winner decides the next location
          (`GameplayStatics.OpenLevel` (`KismetStringLibrary.Conv_StringToName` (`|GetEnumeratorNameAsString` (cast `/Game/VotingObjects/Enums/Enum_Levels` (`KismetMathLibrary.Conv_IntToByte` (- (`/Game/ThirdPerson/Blueprints/GI_ThirdPersonGameInstance.Get Vote Winner` (`self.As GI Third Person Game Instance`)) 1))))))))
      ;[0 0 0] Resets values when Player progresses to next level
      (`/Game/ThirdPerson/Blueprints/GI_ThirdPersonGameInstance.Progress Level` (`self.As GI Third Person Game Instance`)))))

(fn `UserConstructionScript`)