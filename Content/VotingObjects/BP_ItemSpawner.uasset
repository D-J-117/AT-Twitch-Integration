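; BP_ItemSpawner is a rotating text display that shows the item name chosen by an Item vote; it does not spawn anything itself.
; Each Tick spins the text and polls the Game Instance for the vote type and winner.
; A valid winner sets the text from the Items enum, with a tie picking a random entry.
; An Editable flag locks the result until the vote type changes, so random picks don't reroll.
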(event `self.ReceiveBeginPlay`
  ;[0 0 0] Gets Game Instance for later use
  (bind _asgi_third_person_game_instance (cast `/Game/ThirdPerson/Blueprints/GI_ThirdPersonGameInstance` (`GameplayStatics.GetGameInstance`)))
  (set `self.As GI Third Person Game Instance` _asgi_third_person_game_instance))

(event `self.ReceiveTick`
  (params (DeltaSeconds :type "Float (single-precision)"))
  (bind _as_gi_third_person_game_instance (`self.As GI Third Person Game Instance`))
  (bind _vote_winner (`/Game/ThirdPerson/Blueprints/GI_ThirdPersonGameInstance.Get Vote Winner` (`self.As GI Third Person Game Instance`)))
  (`SceneComponent.K2_AddRelativeRotation` (`self.Text`) (* (struct :`Yaw` 50.0) DeltaSeconds) false false)
  (if (and (== (`/Game/ThirdPerson/Blueprints/GI_ThirdPersonGameInstance.Get Current Vote Type` _as_gi_third_person_game_instance) 2) (!= (`/Game/ThirdPerson/Blueprints/GI_ThirdPersonGameInstance.Get Vote Winner` _as_gi_third_person_game_instance) -1))
    (if (`self.Editable`)
      (set `self.Editable` false)
      (if (== _vote_winner 0)
        ;[0 0 0] Tie results in random outcome
        (`TextRenderComponent.K2_SetText` (`self.Text`) (`KismetTextLibrary.Conv_StringToText` (`|GetEnumeratorNameAsString` (cast `/Game/VotingObjects/Enums/Enum_Items` (`KismetMathLibrary.Conv_IntToByte` (`KismetMathLibrary.RandomIntegerInRange` 1 (- (enumcount `/Game/VotingObjects/Enums/Enum_Items`) 1)))))))
        (else
          (`TextRenderComponent.K2_SetText` (`self.Text`) (`KismetTextLibrary.Conv_StringToText` (`|GetEnumeratorNameAsString` (cast `/Game/VotingObjects/Enums/Enum_Items` (`KismetMathLibrary.Conv_IntToByte` _vote_winner))))))))
    (else
      ;[0 0 0] Stops the text from being updated after being assigned. Prevents error with random option
      (if (!= (`/Game/ThirdPerson/Blueprints/GI_ThirdPersonGameInstance.Get Current Vote Type` (`self.As GI Third Person Game Instance`)) 2)
        (set `self.Editable` true)))))

(fn `UserConstructionScript`)