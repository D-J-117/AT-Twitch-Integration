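; Portal actor that teleports the player character to one of several destination actors based on the result of a vote.
; Tick activates the portal and shows its effect only while the game instance reports an Item-type vote with a valid winner.
; Overlapping an active portal teleports the character to the winner's indexed destination, or to a random one when the vote is tied.
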(event `self.ReceiveBeginPlay`
  ;[0 0 0] Gets Game Instance for later use
  (bind _asgi_third_person_game_instance (cast `/Game/ThirdPerson/Blueprints/GI_ThirdPersonGameInstance` (`GameplayStatics.GetGameInstance`)))
  (set `self.As GI Third Person Game Instance` _asgi_third_person_game_instance))

(event `self.ReceiveActorBeginOverlap`
  (params (OtherActor :type "Actor Object Reference"))
  (bind _vote_winner (`/Game/ThirdPerson/Blueprints/GI_ThirdPersonGameInstance.Get Vote Winner` (`self.As GI Third Person Game Instance`)))
  (bind _returnvalue_location (`KismetMathLibrary.BreakTransform` (`self.GetTransform` (`KismetArrayLibrary.Array_Random` (`self.Destination`)))))
  (bind _returnvalue_location_2 (`KismetMathLibrary.BreakTransform` (`self.GetTransform` (`|GetArrayItem` (`self.Destination`) (- _vote_winner 1)))))
  ;[0 0 0] Checks if there is a valid vote winner.
  (if (`self.Active`)
    (bind _asbp_third_person_character (cast `/Game/ThirdPerson/Blueprints/BP_ThirdPersonCharacter` OtherActor))
    (if (!= (`/Game/ThirdPerson/Blueprints/GI_ThirdPersonGameInstance.Get Vote Winner` (`self.As GI Third Person Game Instance`)) -1)
      ;[0 0 0] If vote is a tie, outcome is random
      (if (== _vote_winner 0)
        (`self.K2_SetActorLocation` _asbp_third_person_character _returnvalue_location false true)
        (else
          ;[0 0 0] Otherwise the vote winner decides the next location
          (`self.K2_SetActorLocation` _asbp_third_person_character _returnvalue_location_2 false true))))))

(event `self.ReceiveTick`
  (params (DeltaSeconds :type "Float (single-precision)"))
  (bind _as_gi_third_person_game_instance (`self.As GI Third Person Game Instance`))
  (if (and (== (`/Game/ThirdPerson/Blueprints/GI_ThirdPersonGameInstance.Get Current Vote Type` _as_gi_third_person_game_instance) 1) (!= (`/Game/ThirdPerson/Blueprints/GI_ThirdPersonGameInstance.Get Vote Winner` _as_gi_third_person_game_instance) -1))
    (set `self.Active` true)
    (`SceneComponent.SetVisibility` (`self.Effect`) true false)
    (else
      (set `self.Active` false)
      (`SceneComponent.SetVisibility` (`self.Effect`) false false))))

(fn `UserConstructionScript`)